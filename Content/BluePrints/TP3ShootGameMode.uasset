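; Third-person shooter game mode that spawns the player, allied AI and other AI characters for a given team.
; SpawnNewActor branches on the passed actor's Player or Ally tag, spawns the matching character at a hard-coded location and sets its TeamID.
; Player controller 0 possesses the player character, while each AI character gets a newly spawned controller.
; Allies share the player's spawn point; other AI spawn elsewhere.
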(fn ConstructionScript)

(fn SpawnNewActor
  (params (TeamID :type Generic%20Team%20Id%20Structure) (Actor%20Class :type Actor%20Object%20Reference))
  (if (Actor|ActorHasTag Actor%20Class "Player")
    (bind _returnvalue (Game|SpawnActorfromClass "/Game/ThirdPerson/Blueprints/BP_ThirdPersonCharacter.BP_ThirdPersonCharacter_C" (Math|Transform|MakeTransform "2520.000000,3180.000000,160.000000" "0, 0, 0" "1.000000,1.000000,1.000000") "Undefined" "MultiplyWithRoot" 0 0))
    (Variables|/Script/TP3Shoot.TP3ShootCharacter|SetTeamID _returnvalue TeamID)
    (Pawn|Possess (Game|GetPlayerController 0) _returnvalue)
    (elif (Actor|ActorHasTag Actor%20Class "Ally")
      (bind _output_get (Variables|Default|SetLocalisation1 "2520.000000,3180.000000,160.000000"))
      (bind _returnvalue_2 (Game|SpawnActorfromClass "/Game/Game/Character/BP_AICharacterAlly.BP_AICharacterAlly_C" (Math|Transform|MakeTransform _output_get "0, 0, 0" "1.000000,1.000000,1.000000") "AlwaysSpawn" "MultiplyWithRoot" 0 0))
      (Variables|/Script/TP3Shoot.TP3ShootCharacter|SetTeamID _returnvalue_2 TeamID)
      (bind _returnvalue_3 (Game|SpawnActorfromClass "/Game/Game/Character/BP_AIControllerAlly.BP_AIControllerAlly_C" (Math|Transform|MakeTransform _output_get "0, 0, 0" "1.000000,1.000000,1.000000") "Undefined" "MultiplyWithRoot" 0 0))
      (Pawn|Possess _returnvalue_3 _returnvalue_2)
      (else
        (bind _output_get_2 (Variables|Default|SetLocalisation2 "590.000000,640.000000,160.000000"))
        (bind _returnvalue_4 (Game|SpawnActorfromClass "/Game/Game/Character/BP_AICharacter.BP_AICharacter_C" (Math|Transform|MakeTransform _output_get_2 "0, 0, 0" "1.000000,1.000000,1.000000") "AlwaysSpawn" "MultiplyWithRoot" 0 0))
        (Variables|/Script/TP3Shoot.TP3ShootCharacter|SetTeamID _returnvalue_4 TeamID)
        (bind _returnvalue_5 (Game|SpawnActorfromClass "/Game/Game/Character/BP_AIController.BP_AIController_C" (Math|Transform|MakeTransform _output_get_2 "0, 0, 0" "1.000000,1.000000,1.000000") "Undefined" "MultiplyWithRoot" 0 0))
        (Pawn|Possess _returnvalue_5 _returnvalue_4)))))