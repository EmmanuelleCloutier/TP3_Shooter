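; AI controller for ally characters that turns perception updates into a TargetActor blackboard key.
; A successful sight stimulus stores the sensed actor and prints a debug string, provided the controller itself has the "Ennemi" tag, as the check targets self.
; Lost sight or any non-sight sense clears the key.
; The RunBehaviorTree call for BP_FindCover is unconnected, so this graph never starts a tree.
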(event OnTargetPerceptionUpdated(AIPerception)
  (params (Actor :type Actor%20Object%20Reference) (Stimulus :type AI%20Stimulus%20Structure))
  (bind _returnvalue (Class|AIPerceptionSystem|GetSenseClassforStimulus Stimulus))
  (if (== _returnvalue "/Script/AIModule.AISense_Sight")
    (if (.bSuccessfullySensed (Utilities|Struct|BreakAIStimulus Stimulus))
      (if (Actor|ActorHasTag "Ennemi")
        (Development|PrintString "a to e" true true "(R=0.366956,G=1.000000,B=0.286021,A=1.000000)")
        (AI|Components|Blackboard|SetValueasObject (AI|GetBlackboard 0) (Utilities|Name|MakeLiteralName "TargetActor") Actor))
      (else
        (AI|Components|Blackboard|SetValueasObject (AI|GetBlackboard 0) (Utilities|Name|MakeLiteralName "TargetActor") 0 :!label _label)))
    (else
      (goto _label))))

(event EventBeginPlay)

(fn ConstructionScript)