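; Ally AI character Blueprint for a third-person shooter, with team identity and respawning on destruction.
; On BeginPlay it binds to its own destroyed event, which asks TP3ShootGameMode to spawn a new actor, passing its TeamID and self.
; Aiming toggles walk speed and plays or reverses a timeline that shortens the camera boom.
; An interface function exposes the TeamID.
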(event Custom|OnAim
  (params (bIsAiming :type Boolean))
  (bind _charactermovement (Variables|Character|GetCharacterMovement))
  (if bIsAiming
    (Variables|/Script/Engine.CharacterMovementComponent|SetMaxWalkSpeed _charactermovement 2e+02)
    (bind _newtrack_0 (Timeline|Aiming Play)
      (:Update
        (Variables|/Script/Engine.SpringArmComponent|SetTargetArmLength (Variables|Default|GetCameraBoom) (Math|Float|Lerp 4e+02 2e+02 _newtrack_0))))
    (else
      (Variables|/Script/Engine.CharacterMovementComponent|SetMaxWalkSpeed _charactermovement 5e+02)
      (Timeline|Aiming Reverse))))

(event Custom|OnDestroyed_Event
  (params (DestroyedActor :type Actor%20Object%20Reference))
  (bind _astp3shoot_game_mode (Utilities|Casting|CastToTP3ShootGameMode (Game|GetGameMode)))
  (Default|SpawnNewActor _astp3shoot_game_mode (Variables|Default|GetTeam%20ID) self))

(event EventBeginPlay
  (Game|AssignOnDestroyed (delegate Custom|OnDestroyed_Event)))

(fn ConstructionScript)

(fn BPIGetTeamID
  (return (Variables|Default|GetTeam%20ID)))