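; AI character Blueprint for the shooter, with a team ID exposed through a GetTeamID interface function.
; On destruction it asks the TP3Shoot game mode to spawn a new actor, passing its team ID and itself as the class input.
; Hit events update a HealthBarAI widget with current and max health.
; Aiming slows movement, disables orient-to-movement and uses a timeline to shorten the camera boom, reversing on release.
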(event Custom|OnAim
  (params (bIsAiming :type Boolean))
  (bind _charactermovement (Variables|Character|GetCharacterMovement))
  (bind _charactermovement_2 (Variables|Character|GetCharacterMovement))
  (if bIsAiming
    (Variables|/Script/Engine.CharacterMovementComponent|SetMaxWalkSpeed _charactermovement_2 2e+02)
    (Variables|/Script/Engine.CharacterMovementComponent|SetbOrientRotationToMovement _charactermovement false)
    (bind _newtrack_0 (Timeline|Aiming Play)
      (:Update
        (Variables|/Script/Engine.SpringArmComponent|SetTargetArmLength (Variables|Default|GetCameraBoom) (Math|Float|Lerp 4e+02 2e+02 _newtrack_0))))
    (else
      (Variables|/Script/Engine.CharacterMovementComponent|SetMaxWalkSpeed _charactermovement_2 5e+02)
      (Variables|/Script/Engine.CharacterMovementComponent|SetbOrientRotationToMovement _charactermovement true)
      (Timeline|Aiming Reverse))))

(event Custom|OnDestroyed_Event
  (params (DestroyedActor :type Actor%20Object%20Reference))
  (bind _astp3shoot_game_mode (Utilities|Casting|CastToTP3ShootGameMode (Game|GetGameMode)))
  (Default|SpawnNewActor _astp3shoot_game_mode (Variables|Default|GetTeamID) self))

(event Custom|CustomEvent
  (params (NewHealth :type Float%20%28single-precision%29) (MaxHealth :type Float%20%28single-precision%29))
  (bind _ashealth_bar_ai (Utilities|Casting|CastToHealthBarAI (UserInterface|GetWidget (Variables|Default|GetHealthBar))))
  (Default|SetProgress _ashealth_bar_ai NewHealth MaxHealth))

(event EventBeginPlay
  (Game|AssignOnDestroyed (delegate Custom|OnDestroyed_Event))
  (EventDispatchers|BindEventtoOnHitEvent (delegate Custom|CustomEvent)))

(fn ConstructionScript)

(fn BPIGetTeamID
  (return (Variables|Default|GetTeamID)))