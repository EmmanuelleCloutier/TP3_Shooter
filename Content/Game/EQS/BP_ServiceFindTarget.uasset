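; Behavior tree service, apparently an unfinished target finder, that scans for nearby pawns on each AI tick.
; The "Ennemi" tag selects the branch: tagged pawns run an unfiltered sphere overlap at the default position, others overlap BP_AICharacter around their own location.
; Both branches print debug text regardless of results and loop over the found actors with empty bodies, so no target is stored.
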(event EventReceiveTickAI
  (params (OwnerController :type AI%20Controller%20Object%20Reference) (ControlledPawn :type Pawn%20Object%20Reference) (DeltaSeconds :type Float%20%28single-precision%29))
  (bind _array (Utilities|Array|MakeArray "ObjectTypeQuery3"))
  (Development|PrintString (Utilities|GetDisplayName ControlledPawn) true true "(R=1.000000,G=1.000000,B=1.000000,A=1.000000)")
  (if (Actor|ActorHasTag ControlledPawn "Ennemi")
    (bind _outactors (Collision|SphereOverlapActors "0, 0, 0" 2e+03 _array 0))
    (Development|PrintString "ally or player detected" true true "(R=1.000000,G=0.237566,B=0.207717,A=1.000000)")
    (for _array_element _outactors
      _)
    (else
      (bind _outactors_2 (Collision|SphereOverlapActors (Transformation|GetActorLocation ControlledPawn) 2e+03 _array "/Game/Game/Character/BP_AICharacter.BP_AICharacter_C"))
      (Development|PrintString "ennemi detected" true true "(R=0.273741,G=0.900184,B=1.000000,A=1.000000)")
      (for _array_element_2 _outactors_2
        _))))