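; Behavior tree task that makes a BP_AICharacter face and fire at its blackboard Target when within ShootRange.
; In range it snaps yaw to the target and fires; since IsAiming is set before it is checked, OnAim(true) is never reached.
; Out of range it stops aiming; both branches wait briefly, then finish with IsAiming as the result.
; An invalid target stops aiming and immediately reports success.
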(event EventReceiveExecuteAI
  (params (OwnerController :type AI%20Controller%20Object%20Reference) (ControlledPawn :type Pawn%20Object%20Reference))
  (bind _target (Variables|Default|GetTarget))
  (bind _returnvalue (AI|BehaviorTree|GetBlackboardValueasActor _target))
  (if (Utilities|IsValid _returnvalue)
    (bind _asbp_aicharacter (Utilities|Casting|CastToBP_AICharacter ControlledPawn))
    (if (<= (Transformation|GetDistanceTo ControlledPawn _returnvalue) (Variables|Default|GetShootRange))
      (bind _output_get (Variables|/Script/TP3Shoot.TP3ShootCharacter|SetIsAiming _asbp_aicharacter true))
      (Transformation|SetActorRotation _asbp_aicharacter (Math|Rotator|MakeRotator (.roll (Transformation|GetActorRotation _asbp_aicharacter)) (.pitch (Transformation|GetActorRotation _asbp_aicharacter)) (.yaw (Math|Rotator|FindLookatRotation (Transformation|GetActorLocation ControlledPawn) (Transformation|GetActorLocation _returnvalue)))) true)
      (if (Variables|/Script/TP3Shoot.TP3ShootCharacter|GetIsAiming _asbp_aicharacter)
        _
        (else
          (Default|OnAim _asbp_aicharacter true)))
      (Class|TP3ShootCharacter|Fire _asbp_aicharacter)
      (Utilities|FlowControl|Delay 0.5)
      (else
        (Variables|/Script/TP3Shoot.TP3ShootCharacter|SetIsAiming _asbp_aicharacter false)
        (Default|OnAim _asbp_aicharacter false)
        (Utilities|FlowControl|Delay 0.5)))
    (AI|BehaviorTree|FinishExecute _output_get)
    (else
      (bind _asbp_aicharacter_2 (Utilities|Casting|CastToBP_AICharacter ControlledPawn))
      (Variables|/Script/TP3Shoot.TP3ShootCharacter|SetIsAiming _asbp_aicharacter_2 false)
      (Default|OnAim _asbp_aicharacter_2 false)
      (AI|BehaviorTree|FinishExecute true))))